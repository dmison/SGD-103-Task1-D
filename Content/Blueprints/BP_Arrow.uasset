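; BP_Arrow is an arrow projectile that damages actors it overlaps.
; On sphere overlap it skips itself, sends one point of damage through TakeDamageMessage with a launch at half its horizontal velocity plus a small upward boost, then destroys itself.
; A blocking hit on the sphere destroys the arrow after a short delay.
; The DoHit function and construction script are empty.
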(event OnComponentBeginOverlap(Sphere)
  (params (OverlappedComponent :type Primitive%20Component%20Object%20Reference) (OtherActor :type Actor%20Object%20Reference) (OtherComp :type Primitive%20Component%20Object%20Reference) (OtherBodyIndex :type Integer) (bFromSweep :type Boolean) (SweepResult :type Hit%20Result%20Structure%20%28by%20ref%29))
  (bind _returnvalue (Transformation|GetVelocity))
  ;[1 1 1] don't let an arrow hit itself
  (if (not (Utilities|Enum|Equal(Enum) (Utilities|GetDisplayName self) (Utilities|GetDisplayName OtherActor)))
    (Class|BPIHealth|TakeDamage(Message) OtherActor 1 (Math|Vector|MakeVector (/ (.x _returnvalue) 2.0) (/ (.y _returnvalue) 2.0) 1e+02))
    (Actor|DestroyActor)))

(event OnComponentHit(Sphere)
  (params (HitComponent :type Primitive%20Component%20Object%20Reference) (OtherActor :type Actor%20Object%20Reference) (OtherComp :type Primitive%20Component%20Object%20Reference) (NormalImpulse :type Vector :default "0, 0, 0") (Hit :type Hit%20Result%20Structure%20%28by%20ref%29))
  (Utilities|FlowControl|Delay 1.5)
  (Actor|DestroyActor))

(fn ConstructionScript)

(fn DoHit
  (params (actor :type Actor%20Object%20Reference)))
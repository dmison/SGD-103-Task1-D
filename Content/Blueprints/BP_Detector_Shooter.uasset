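; BP_Detector_Shooter is a trap that fires arrows when the player crosses its line of sight.
; Every tick it sphere-traces on the Camera channel from ArrowSource along its forward vector out to DetectorRange, with persistent debug drawing left on.
; A hit on player character 0 calls ShootArrow, which spawns a BP_Arrow at ArrowSource and plays a sound.
; A DoOnce reset after a Delay acts as the firing cooldown.
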(event Custom|ShootArrow
  (Utilities|FlowControl|DoOnce false :!label _label
    (:Completed
      (Game|SpawnActorfromClass "/Game/Blueprints/BP_Arrow.BP_Arrow_C" (Transformation|GetWorldTransform (Variables|Default|GetArrowSource)) "Undefined" "MultiplyWithRoot" 0 0)
      (Audio|PlaySoundatLocation "/Game/Sounds/Arrow_SFX_Cue.Arrow_SFX_Cue" (Transformation|GetActorLocation) "0, 0, 0" 1.0 1.0 0.2 0 0 0 0)
      (Utilities|FlowControl|Delay 2.0)
      (goto _label Reset))))

(event EventTick
  (params (DeltaSeconds :type Float%20%28single-precision%29))
  (bind _arrowsource (Variables|Default|GetArrowSource))
  (bind _returnvalue (Transformation|GetWorldLocation _arrowsource))
  (bind _outhit (Collision|SphereTraceByChannel _returnvalue (+ _returnvalue (* (Variables|Default|GetDetectorRange) (Math|Vector|GetForwardVector (Transformation|GetWorldRotation _arrowsource)))) 2e+01 "TraceTypeQuery2" false 0 "Persistent"))
  (if (== (.HitActor (Collision|BreakHitResult _outhit)) (Game|GetPlayerCharacter 0))
    (CallFunction|ShootArrow)))

(fn ConstructionScript)
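; BP_KeyPlatform is an interactable platform holding a key that the player can pick up.
; Interact calls AddKeyMessage on the player, destroys the Key component and plays a skull pickup sound at player 0's location.
; GetHint supplies the pickup prompt, and both functions check that Key is still valid, so the pickup works once and the hint then turns blank.
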(event EventInteract
  (params (player :type BP%20Player%20Character%20Object%20Reference))
  (bind _key (Variables|Default|GetKey))
  (Utilities|IsValid _key
    (:Is%20Valid
      (Class|BPIPlayerCharacter|AddKey(Message) player)
      (Components|DestroyComponent _key)
      (Audio|PlaySoundatLocation "/Game/Sounds/PickupSkull_SFX.PickupSkull_SFX" (Transformation|GetActorLocation (Game|GetPlayerCharacter 0)) "0, 0, 0" 2.0 1.0 0.0 0 0 0 0))))

(fn ConstructionScript)

(fn GetHint
  (params (player :type BP%20Player%20Character%20Object%20Reference))
  (Utilities|IsValid (Variables|Default|GetKey)
    (:Is%20Valid
      (return "Press 'E\" to get Key"))
    (:Is%20Not%20Valid
      (return ""))))
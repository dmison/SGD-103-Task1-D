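; Game mode for the maze game that owns the HUD and handles the win and lose end states.
; BeginPlay creates the heads-up display widget and adds it to the viewport.
; Lose and WinEvent each disable player input, fade the camera to a red or white tint, and remove the HUD.
; After a short delay, they show the matching end screen with UI-only input and a visible cursor.
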(event Custom|Lose
  (bind _returnvalue (Game|GetPlayerController 0))
  ;[1 1 1] You Lose the Game
  (Input|DisableInput (Game|GetPlayerCharacter 0) (Game|GetPlayerController 0))
  (CameraFades|StartCameraFade (Game|GetPlayerCameraManager 0) 0.0 0.8 2.0 "(R=0.265625,G=0.000000,B=0.013664,A=1.000000)" false true)
  (Widget|RemovefromParent (Variables|Default|GetHeadsUpDisplay))
  (Utilities|FlowControl|Delay 1.0)
  (bind _returnvalue_2 (UserInterface|CreateWidget "/Game/UI/WBP_LoseScreen.WBP_LoseScreen_C"))
  (UserInterface|Viewport|AddtoViewport _returnvalue_2 0)
  (Input|SetInputModeUIOnly _returnvalue _returnvalue_2 "DoNotLock" false)
  (Variables|/Script/Engine.PlayerController|SetbShowMouseCursor _returnvalue true))

(event Custom|WinEvent
  (bind _returnvalue (Game|GetPlayerController 0))
  (Input|DisableInput (Game|GetPlayerCharacter 0) (Game|GetPlayerController 0))
  (CameraFades|StartCameraFade (Game|GetPlayerCameraManager 0) 0.0 0.8 2.0 "(R=1.000000,G=0.985269,B=0.996317,A=1.000000)" false true)
  (Widget|RemovefromParent (Variables|Default|GetHeadsUpDisplay))
  (Utilities|FlowControl|Delay 0.5)
  (bind _returnvalue_2 (UserInterface|CreateWidget "/Game/UI/WBP_WinScreen1.WBP_WinScreen1_C"))
  (UserInterface|Viewport|AddtoViewport _returnvalue_2 0)
  (Input|SetInputModeUIOnly _returnvalue 0 "DoNotLock" false)
  (Variables|/Script/Engine.PlayerController|SetbShowMouseCursor _returnvalue true))

(event EventBeginPlay
  ;[1 1 1] Add HUD
  (bind _returnvalue (UserInterface|CreateWidget "/Game/UI/WBP_HeadsUpDisplay.WBP_HeadsUpDisplay_C"))
  (bind _output_get (Variables|Default|SetHeadsUpDisplay _returnvalue))
  (UserInterface|Viewport|AddtoViewport _output_get 0))

(fn ConstructionScript)
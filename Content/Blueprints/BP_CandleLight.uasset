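; Candle light actor that gives its point light a randomized flicker.
; On BeginPlay it creates a dynamic instance of MI_Flicker, randomizes its FlickerTime and LowestBrightness parameters once, and assigns it as the PointLight's light function material.
; The flicker itself comes from that material, since Tick is empty and a second, wider-range randomization is left unconnected.
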(event EventBeginPlay
  (bind _returnvalue (Rendering|Material|CreateDynamicMaterialInstance "/Game/Materials/MI_Flicker.MI_Flicker" "CustomFlicker" "None" :!class /Script/Engine.KismetMaterialLibrary))
  (bind _output_get (Variables|Default|SetFlickerMI _returnvalue))
  (Rendering|Material|SetScalarParameterValue _output_get "FlickerTime" (Math|Random|RandomFloatinRange 0.5 1.0) :!class /Script/Engine.MaterialInstanceDynamic)
  (Rendering|Material|SetScalarParameterValue _output_get "LowestBrightness" (Math|Random|RandomFloatinRange 0.5 1.0) :!class /Script/Engine.MaterialInstanceDynamic)
  (Rendering|Components|Light|SetLightFunctionMaterial (Variables|Default|GetPointLight) _output_get))

(event Collision|EventActorBeginOverlap
  (params (OtherActor :type Actor%20Object%20Reference)))

(event EventTick
  (params (DeltaSeconds :type Float%20%28single-precision%29)))

(fn ConstructionScript)
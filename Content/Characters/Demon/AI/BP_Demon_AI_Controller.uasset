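; AI controller for the Demon character that runs BT_Demon on BeginPlay and feeds its blackboard from AI perception.
; A CanSeePlayer helper accepts only successful sight stimuli from player character 0, which set TargetActor.
; Any other target update clears TargetActor and writes an empty object to LastKnownLocation; the vector write of the actor's location is unconnected.
; General perception updates only print the updated actor count for debugging.
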(event OnPerceptionUpdated(AIPerception)
  (params (UpdatedActors :type Array%20of%20Actor%20Object%20References))
  (Development|PrintString (Utilities|String|ToString(Integer) (Utilities|Array|Length UpdatedActors))))

(event OnTargetPerceptionUpdated(AIPerception)
  (params (Actor :type Actor%20Object%20Reference) (Stimulus :type AI%20Stimulus%20Structure))
  (bind _result (CallFunction|CanSeePlayer Actor Stimulus))
  (if _result
    (AI|Components|Blackboard|SetValueasObject (Variables|Default|GetBlackboard) (Utilities|Name|MakeLiteralName "TargetActor") Actor)
    (else
      (AI|Components|Blackboard|ClearValue (Variables|Default|GetBlackboard) (Utilities|Name|MakeLiteralName "TargetActor"))
      (AI|Components|Blackboard|SetValueasObject (Variables|Default|GetBlackboard) (Utilities|Name|MakeLiteralName "LastKnownLocation") 0))))

(event EventBeginPlay
  (AI|RunBehaviorTree "/Game/Characters/Demon/AI/BT_Demon.BT_Demon"))

(fn ConstructionScript)

(fn CanSeePlayer
  (params (Actor :type Actor%20Object%20Reference%20%28by%20ref%29) (Stimulus :type AI%20Stimulus%20Structure%20%28by%20ref%29))
  (bind _returnvalue (Class|AIPerceptionSystem|GetSenseClassforStimulus Stimulus))
  (return (Math|Boolean|ANDBoolean (== _returnvalue "/Script/AIModule.AISense_Sight") (== Actor (Game|GetPlayerCharacter 0)) (.bsuccessfullysensed Stimulus))))
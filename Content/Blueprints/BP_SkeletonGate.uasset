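; Interactable skeleton gate that opens when the player has a key, with a hint about the missing head while closed.
; Interact calls the player's UseKeyMessage, spawns a key mesh at SkullPlace, and plays a timeline that slides it and swings both gate halves.
; On finish, the chains are destroyed and the key and skeleton parts switch to physics simulation individually.
; Interact never checks IsOpen, so it can retrigger.
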(event EventInteract
  (params (player :type Object%20Object%20Reference))
  (bind _asbp_player_character (Utilities|Casting|CastToBP_PlayerCharacter player))
  (if (> (Variables|/Game/Characters/Player/BP_PlayerCharacter.BP_PlayerCharacter_C|GetNumberOfKeys _asbp_player_character) 0)
    (Variables|Default|SetIsOpen true)
    (Class|BPIPlayerCharacter|UseKey(Message) player)
    (bind _returnvalue (AddComponent|AddStaticMeshComponent false))
    (bind _output_get (Variables|Default|SetKeyMesh _returnvalue))
    (Transformation|AttachComponentToComponent _output_get (Variables|Default|GetSkullPlace) "None" "SnapToTarget" "KeepWorld" "SnapToTarget" true)
    (bind (_direction _door_position _key_position) (Timeline|Timeline PlayFromStart)
      (:Update
        (Transformation|SetRelativeLocation (Variables|Default|GetKeyMesh) (Math|Vector|MakeVector 0.0 _key_position 0.0) false false)
        (Transformation|SetRelativeRotation (Variables|Default|GetSM_Plains_CastleArch_Iron_Gate_02) (Math|Rotator|MakeRotator 0.0 0.0 (* _door_position -1.0)) false false)
        (Transformation|SetRelativeRotation (Variables|Default|GetSM_Plains_CastleArch_Iron_Gate_03) (Math|Rotator|MakeRotator 0.0 0.0 (+ _door_position -1.8e+02)) false false))
      (:Finished
        ;[1 1 1] This is rediculous why does the get children not work correctly?
        (Physics|SetSimulatePhysics (Variables|Default|GetSkeletonTorso) true)
        (Physics|SetSimulatePhysics (Variables|Default|GetKeyMesh) true)
        (Physics|SetSimulatePhysics (Variables|Default|GetSkeletonArm) true)
        (Physics|SetSimulatePhysics (Variables|Default|GetSkeletonArm1) true)
        (Physics|SetSimulatePhysics (Variables|Default|GetSkeletonLeg) true)
        (Physics|SetSimulatePhysics (Variables|Default|GetSkeletonLeg1) true)
        (Components|DestroyComponent (Variables|Default|GetSM_Env_Fire_deco_Chain2))
        (Components|DestroyComponent (Variables|Default|GetSM_Env_Fire_deco_Chain1))))))

(fn ConstructionScript)

(fn GetHint
  (params (player :type Object%20Object%20Reference))
  (if (not (Variables|Default|GetIsOpen))
    (return "Looks like this guy lost his head over something")
    (else
      (return ""))))
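; BP_FireBolt is a fire projectile that explodes on impact and damages what it hits.
; On Sphere hit, it sets the point light's intensity, spawns explosion particles and sound at the impact point, and destroys components such as its trails.
; It sends the hit actor a damage message with a launch vector built from half its horizontal velocity plus fixed lift.
; A short timer delays destroying the actor.
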(event OnComponentBeginOverlap(Sphere)
  (params (OverlappedComponent :type Primitive%20Component%20Object%20Reference) (OtherActor :type Actor%20Object%20Reference) (OtherComp :type Primitive%20Component%20Object%20Reference) (OtherBodyIndex :type Integer) (bFromSweep :type Boolean) (SweepResult :type Hit%20Result%20Structure%20%28by%20ref%29)))

(event OnComponentHit(Sphere)
  (params (HitComponent :type Primitive%20Component%20Object%20Reference) (OtherActor :type Actor%20Object%20Reference) (OtherComp :type Primitive%20Component%20Object%20Reference) (NormalImpulse :type Vector :default "0, 0, 0") (Hit :type Hit%20Result%20Structure%20%28by%20ref%29))
  (bind _returnvalue (Transformation|GetVelocity))
  (bind _location (Collision|BreakHitResult Hit))
  (Rendering|Components|Light|SetIntensity (Variables|Default|GetPointLight) 6e+03)
  (Effects|SpawnEmitteratLocation "/Game/StarterContent/Particles/P_Explosion.P_Explosion" _location)
  (Audio|PlaySoundatLocation "/Game/Sounds/medium-explosion-40472_Cue.medium-explosion-40472_Cue" _location "0, 0, 0" 1.0 1.0 0.0 0 0 0 0)
  (for _array_element (Utilities|Array|MakeArray (Variables|Default|GetSphere2) (Variables|Default|Gettrail1) (Variables|Default|Gettrail) 0)
    (Utilities|IsValid _array_element
      (:Is%20Valid
        (Components|DestroyComponent _array_element))))
  (Class|BPIHealth|TakeDamage(Message) OtherActor 30 (Math|Vector|MakeVector (/ (.x _returnvalue) 2.0) (/ (.y _returnvalue) 2.0) 1e+02))
  (Utilities|Time|SetTimerbyEvent (delegate Custom|CustomEvent) 0.2))

(event Custom|CustomEvent
  (Actor|DestroyActor))

(fn ConstructionScript)
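; BP_Elevator is an elevator actor that moves vertically when something overlaps its trigger volume.
; It records its starting height on BeginPlay, then on overlap disables the trigger's overlap events, waits briefly and plays a timeline from the start.
; The timeline track, scaled by Distance, offsets Z from that height through a relative-location set fed with world coordinates.
; Overlap events are re-enabled when the timeline finishes.
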(event OnComponentBeginOverlap(TriggerVolume)
  (params (OverlappedComponent :type Primitive%20Component%20Object%20Reference) (OtherActor :type Actor%20Object%20Reference) (OtherComp :type Primitive%20Component%20Object%20Reference) (OtherBodyIndex :type Integer) (bFromSweep :type Boolean) (SweepResult :type Hit%20Result%20Structure%20%28by%20ref%29))
  (bind _returnvalue (Transformation|GetActorLocation))
  (bind _trigger_volume (Variables|Default|GetTrigger%20Volume))
  (Variables|/Script/Engine.PrimitiveComponent|SetbGenerateOverlapEvents _trigger_volume false)
  (Utilities|FlowControl|Delay 2.0)
  (bind _newtrack_1 (Timeline|Timeline PlayFromStart)
    (:Update
      (Transformation|SetActorRelativeLocation (Math|Vector|MakeVector (.x _returnvalue) (.y _returnvalue) (+ (* _newtrack_1 (/ (Variables|Default|GetDistance) 1e+02)) (Variables|Default|GetStartZ)))))
    (:Finished
      (Variables|/Script/Engine.PrimitiveComponent|SetbGenerateOverlapEvents _trigger_volume true))))

(event EventBeginPlay
  (Variables|Default|SetStartZ (.z (Transformation|GetActorLocation))))

(fn ConstructionScript)
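; BP_Demon is a demon AI character that takes damage and ragdolls on death.
; BeginPlay stores its starting location and rotation as its home transform.
; TakeDamage subtracts from Health and, at zero or below, switches the mesh to physics simulation, then stops the AI controller's brain logic and disables its sight sense.
; The CurrentHealth function is a stub that returns zero rather than reading Health.
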(event EventTakeDamage
  (params (amount :type Integer) (launch :type Vector :default "0, 0, 0"))
  (bind _returnvalue (AI|GetAIController 0))
  (bind _mesh (Variables|Character|GetMesh))
  ;[0.349 0 0] Take Damage
  ;;[1 1 1] update health
  (bind _output_get (Variables|Default|SetHealth (- (Variables|Default|GetHealth) amount)))
  ;;[1 1 1] am I dead?
  (if (<= _output_get 0)
    ;;[1 1 1] rag doll me
    (Collision|SetCollisionEnabled _mesh "PhysicsOnly")
    (Physics|SetSimulatePhysics _mesh true)
    ;;[1 1 1] stop behaviour tree
    (Utilities|IsValid _returnvalue
      (:Is%20Valid
        (AI|Logic|StopLogic (Variables|/Script/AIModule.AIController|GetBrainComponent _returnvalue) "")
        ;;[1 1 1] stop sight
        (Utilities|IsValid _returnvalue
          (:Is%20Valid
            (Class|AIPerceptionComponent|SetSenseEnabled (Class|AIController|GetAIPerceptionComponent _returnvalue) "/Script/AIModule.AISense_Sight" false)))))))

(event EventBeginPlay
  (Variables|Default|SetHomeLocation (Transformation|GetActorLocation))
  (Variables|Default|SetHomeRotation (Transformation|GetActorRotation)))

(fn ConstructionScript)

(fn CurrentHealth
  (return 0))
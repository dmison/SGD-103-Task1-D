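; BP_Door is a locked door that opens when a player with at least one key interacts with it.
; The Interact event takes one key from the player, creates a key mesh component at runtime and attaches it to the Keyhole.
; The OpenDoor timeline then drives the key's relative X position and the door mesh's relative Z position.
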(event EventInteract
  (params (player :type BP%20Player%20Character%20Object%20Reference))
  (bind _numberofkeys (Variables|/Game/Player/BP_PlayerCharacter.BP_PlayerCharacter_C|GetNumberOfKeys player))
  (if (> _numberofkeys 0)
    (Math|Integer|DecrementInt _numberofkeys
      (:%20%20
        (bind _returnvalue (AddComponent|AddStaticMeshComponent false))
        (bind _output_get (Variables|Default|SetKeyMesh _returnvalue))
        (Transformation|AttachComponentToComponent _output_get (Variables|Default|GetKeyhole) "None" "SnapToTarget" "KeepWorld" "SnapToTarget" true)
        (bind (_direction _door_position _key_position) (Timeline|OpenDoor PlayFromStart)
          (:Update
            (Transformation|SetRelativeLocation (Variables|Default|GetKeyMesh) (Math|Vector|MakeVector _key_position 0.0 0.0) false false)
            (Transformation|SetRelativeLocation (Variables|Default|GetDoorMesh) (Math|Vector|MakeVector 0.0 0.0 _door_position) false false)))))))

(fn ConstructionScript)
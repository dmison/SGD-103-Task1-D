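; Player character for a maze game, handling movement, interaction, key counting, fire bolt shooting and damage.
; Enhanced Input drives camera-relative movement, with DoOnce-plus-Delay gates throttling footstep sounds and shots.
; The InteractionSpace volume fetches hint text on overlap and sends interact messages to overlapping actors.
; Key and health changes update the HUD through BP_MazeGameMode; damage also launches the player and triggers Lose at zero health.
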(event OnComponentBeginOverlap(InteractionSpace)
  (params (OverlappedComponent :type Primitive%20Component%20Object%20Reference) (OtherActor :type Actor%20Object%20Reference) (OtherComp :type Primitive%20Component%20Object%20Reference) (OtherBodyIndex :type Integer) (bFromSweep :type Boolean) (SweepResult :type Hit%20Result%20Structure%20%28by%20ref%29))
  ;[1 1 1] get interaction hint
  (bind _asbp_player_character (Utilities|Casting|CastToBP_PlayerCharacter (Game|GetPlayerCharacter 0)))
  (bind _text (Class|BPIInteract|GetHint(Message) OtherActor _asbp_player_character))
  (bind _asbp_maze_game_mode (Utilities|Casting|CastToBP_MazeGameMode (Game|GetGameMode)))
  (Rendering|Components|TextRender|SetText (Variables|/Game/UI/WBP_HeadsUpDisplay.WBP_HeadsUpDisplay_C|GetHintText (Variables|/Game/GameSettings/BP_MazeGameMode.BP_MazeGameMode_C|GetHeadsUpDisplay _asbp_maze_game_mode)) (Utilities|Text|ToText(String) _text)))

(event OnComponentEndOverlap(InteractionSpace)
  (params (OverlappedComponent :type Primitive%20Component%20Object%20Reference) (OtherActor :type Actor%20Object%20Reference) (OtherComp :type Primitive%20Component%20Object%20Reference) (OtherBodyIndex :type Integer))
  ;[1 1 1] update interaction hint
  (bind _asbp_maze_game_mode (Utilities|Casting|CastToBP_MazeGameMode (Game|GetGameMode)))
  (Rendering|Components|TextRender|SetText (Variables|/Game/UI/WBP_HeadsUpDisplay.WBP_HeadsUpDisplay_C|GetHintText (Variables|/Game/GameSettings/BP_MazeGameMode.BP_MazeGameMode_C|GetHeadsUpDisplay _asbp_maze_game_mode)) ""))

(event Input|EnhancedActionEvents|EnhancedInputActionIA_MoveForward
  (params (ActionValue :type Float%20%28double-precision%29) (ElapsedSeconds :type Float%20%28double-precision%29) (TriggeredSeconds :type Float%20%28double-precision%29) (InputAction :type Input%20Action%20Object%20Reference :default "/Game/Inputs/IA_MoveForward.IA_MoveForward"))
  ;[1 1 1] Movement and Looking
  (Pawn|Input|AddMovementInput (Math|Vector|GetForwardVector (Transformation|GetWorldRotation (Variables|Default|GetCamera))) ActionValue false)
  (if (!= ActionValue 0.0)
    (Utilities|FlowControl|DoOnce false :!label _label
      (:Completed
        (Audio|PlaySoundatLocation "/Game/Sounds/Footstep_SFX.Footstep_SFX" (Transformation|GetActorLocation) "0, 0, 0" 1.0 1.0 0.0 0 0 0 0)
        (Utilities|FlowControl|Delay 0.5)
        (goto _label Reset)))))

(event Input|EnhancedActionEvents|EnhancedInputActionIA_Strafe
  (params (ActionValue :type Float%20%28double-precision%29) (ElapsedSeconds :type Float%20%28double-precision%29) (TriggeredSeconds :type Float%20%28double-precision%29) (InputAction :type Input%20Action%20Object%20Reference :default "/Game/Inputs/IA_Strafe.IA_Strafe"))
  ;[1 1 1] Movement and Looking
  (Pawn|Input|AddMovementInput (Math|Vector|GetRightVector (Transformation|GetWorldRotation (Variables|Default|GetCamera))) ActionValue false)
  (if (!= ActionValue 0.0)
    (Utilities|FlowControl|DoOnce false :!label _label
      (:Completed
        (Audio|PlaySoundatLocation "/Game/Sounds/Footstep_SFX.Footstep_SFX" (Transformation|GetActorLocation) "0, 0, 0" 1.0 1.0 0.0 0 0 0 0)
        (Utilities|FlowControl|Delay 0.5)
        (goto _label Reset)))))

(event Input|EnhancedActionEvents|EnhancedInputActionIA_LookUp
  (params (ActionValue :type Float%20%28double-precision%29) (ElapsedSeconds :type Float%20%28double-precision%29) (TriggeredSeconds :type Float%20%28double-precision%29) (InputAction :type Input%20Action%20Object%20Reference :default "/Game/Inputs/IA_LookUp.IA_LookUp"))
  ;[1 1 1] Movement and Looking
  (Pawn|Input|AddControllerPitchInput ActionValue))

(event Input|EnhancedActionEvents|EnhancedInputActionIA_Turn
  (params (ActionValue :type Float%20%28double-precision%29) (ElapsedSeconds :type Float%20%28double-precision%29) (TriggeredSeconds :type Float%20%28double-precision%29) (InputAction :type Input%20Action%20Object%20Reference :default "/Game/Inputs/IA_Turn.IA_Turn"))
  ;[1 1 1] Movement and Looking
  (Pawn|Input|AddControllerYawInput ActionValue))

(event Input|EnhancedActionEvents|EnhancedInputActionIA_Interact
  (params (ActionValue :type Boolean) (ElapsedSeconds :type Float%20%28double-precision%29) (TriggeredSeconds :type Float%20%28double-precision%29) (InputAction :type Input%20Action%20Object%20Reference :default "/Game/Inputs/IA_Interact.IA_Interact"))
  (:Completed
    ;[1 1 1] Interaction
    (for _array_element (Collision|GetOverlappingActors (Variables|Default|GetInteractionSpace) 0 :!class /Script/Engine.PrimitiveComponent)
      (Class|BPIInteract|Interact(Message) _array_element self))))

(event Input|EnhancedActionEvents|EnhancedInputActionIA_Shoot
  (params (ActionValue :type Boolean) (ElapsedSeconds :type Float%20%28double-precision%29) (TriggeredSeconds :type Float%20%28double-precision%29) (InputAction :type Input%20Action%20Object%20Reference :default "/Game/Inputs/IA_Shoot.IA_Shoot"))
  ;[1 1 1] Shoot
  (Utilities|FlowControl|DoOnce false :!label _label
    (:Completed
      (Game|SpawnActorfromClass "/Game/Blueprints/BP_FireBolt.BP_FireBolt_C" (Transformation|GetWorldTransform (Variables|Default|GetshootSource)) "Undefined" "MultiplyWithRoot" 0 0)
      (Utilities|FlowControl|Delay 0.75)
      (goto _label Reset))))

(event EventBeginPlay
  ;[1 1 1] Setup Inputs
  (Input|AddMappingContext (PlayerController|LocalPlayerSubsystems|GetEnhancedInputLocalPlayerSubsystem (Game|GetPlayerController 0)) "/Game/Inputs/IMC_Default.IMC_Default" 0 "(bIgnoreAllPressedKeysUntilRelease=True,bForceImmediately=False,bNotifyUserSettings=False)"))

(event EventUseKey
  ;[1 1 1] key management
  (bind _result (Math|Integer|DecrementInt (Variables|Default|GetNumberOfKeys))
    (:%20%20
      (Variables|Default|SetNumberOfKeys _result)
      (bind _asbp_maze_game_mode (Utilities|Casting|CastToBP_MazeGameMode (Game|GetGameMode)))
      (Default|UpdateSkulls (Variables|/Game/GameSettings/BP_MazeGameMode.BP_MazeGameMode_C|GetHeadsUpDisplay _asbp_maze_game_mode))
      ;[1 1 1] update interaction hint
      (bind _asbp_maze_game_mode_2 (Utilities|Casting|CastToBP_MazeGameMode (Game|GetGameMode)))
      (Rendering|Components|TextRender|SetText (Variables|/Game/UI/WBP_HeadsUpDisplay.WBP_HeadsUpDisplay_C|GetHintText (Variables|/Game/GameSettings/BP_MazeGameMode.BP_MazeGameMode_C|GetHeadsUpDisplay _asbp_maze_game_mode_2)) ""))))

(event EventAddKey
  ;[1 1 1] key management
  (bind _result (Math|Integer|IncrementInt (Variables|Default|GetNumberOfKeys))
    (:%20%20
      (Variables|Default|SetNumberOfKeys _result)
      (bind _asbp_maze_game_mode (Utilities|Casting|CastToBP_MazeGameMode (Game|GetGameMode)))
      (Default|UpdateSkulls (Variables|/Game/GameSettings/BP_MazeGameMode.BP_MazeGameMode_C|GetHeadsUpDisplay _asbp_maze_game_mode))
      ;[1 1 1] update interaction hint
      (bind _asbp_maze_game_mode_2 (Utilities|Casting|CastToBP_MazeGameMode (Game|GetGameMode)))
      (Rendering|Components|TextRender|SetText (Variables|/Game/UI/WBP_HeadsUpDisplay.WBP_HeadsUpDisplay_C|GetHintText (Variables|/Game/GameSettings/BP_MazeGameMode.BP_MazeGameMode_C|GetHeadsUpDisplay _asbp_maze_game_mode_2)) ""))))

(event EventTakeDamage
  (params (amount :type Integer) (launch :type Vector :default "0, 0, 0"))
  ;[1 1 1] Taking Damage
  (if (> (Variables|Default|GetHealth) 0)
    (Variables|Default|SetHealth (Math|Float|Truncate (- (Variables|Default|GetHealth) (Math|Float|Truncate (Math|Conversions|ToFloat(Integer) amount)))))
    (bind _asbp_maze_game_mode (Utilities|Casting|CastToBP_MazeGameMode (Game|GetGameMode)))
    (Default|UpdateHealth (Variables|/Game/GameSettings/BP_MazeGameMode.BP_MazeGameMode_C|GetHeadsUpDisplay _asbp_maze_game_mode))
    (Audio|PlaySoundatLocation "/Game/Sounds/Hit_SFX.Hit_SFX" (Transformation|GetActorLocation) "0, 0, 0" 1.0 1.0 0.0 0 0 0 0)
    (Character|LaunchCharacter (+ (Transformation|GetVelocity) launch) false false)
    (if (<= (Variables|Default|GetHealth) 0)
      (Default|Lose _asbp_maze_game_mode))))

(fn ConstructionScript)
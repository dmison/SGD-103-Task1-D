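; BP_HealthPotion is an interactable potion that heals the player once.
; On Interact, if the player's health is below 100 and the Potion component is still valid, it sends a 50-point heal, destroys that component and plays a drinking sound at the player character.
; The component's validity doubles as the unused flag, so GetHint shows the "Miracle Cure" label only until the potion is drunk.
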(event EventInteract
  (params (player :type Object%20Object%20Reference))
  (bind _potion (Variables|Default|GetPotion))
  (bind _currenthealth (Class|BPIHealth|CurrentHealth(Message) player))
  (if (< _currenthealth 100)
    (Utilities|IsValid _potion
      (:Is%20Valid
        (Class|BPIHealth|Heal(Message) player 50)
        (Components|DestroyComponent _potion)
        (Audio|PlaySoundatLocation "/Game/Sounds/drink-sip-and-swallow-6974.drink-sip-and-swallow-6974" (Transformation|GetActorLocation (Game|GetPlayerCharacter 0)) "0, 0, 0" 2.0 1.0 0.0 0 0 0 0)))))

(fn ConstructionScript)

(fn GetHint
  (params (player :type Object%20Object%20Reference))
  (Utilities|IsValid (Variables|Default|GetPotion)
    (:Is%20Valid
      (return "The label reads \"Miracle Cure\""))
    (:Is%20Not%20Valid
      (return ""))))
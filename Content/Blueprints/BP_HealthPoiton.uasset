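; BP_HealthPoiton is an interactable health potion that the player drinks to heal.
; Interact sends a heal message to the player, destroys the Potion component and plays a pickup sound at the player's location.
; GetHint returns a drink prompt while the Potion component exists and an empty string afterward, so the same validity check makes it single-use.
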(event EventInteract
  (params (player :type Object%20Object%20Reference))
  (bind _potion (Variables|Default|GetPotion))
  (Utilities|IsValid _potion
    (:Is%20Valid
      (Class|BPIHealth|Heal(Message) player 50)
      (Components|DestroyComponent _potion)
      (Audio|PlaySoundatLocation "/Game/Sounds/PickupSkull_SFX.PickupSkull_SFX" (Transformation|GetActorLocation (Game|GetPlayerCharacter 0)) "0, 0, 0" 2.0 1.0 0.0 0 0 0 0))))

(fn ConstructionScript)

(fn GetHint
  (params (player :type Object%20Object%20Reference))
  (Utilities|IsValid (Variables|Default|GetPotion)
    (:Is%20Valid
      (return "This is labelled \"Miracle Cure\" and contains a glowing liquid.  Press E to drink it"))
    (:Is%20Not%20Valid
      (return ""))))